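; Player Blueprint for a 2D side-scrolling flipbook character that runs, jumps and picks up keys.
; Axis input moves it along X, while Tick flips controller yaw to face travel direction and selects idle, run or falling flipbooks through SetFlipBook.
; Jumping and landing play preloaded 2D sounds and trigger a shared land/jump flipbook with short delays.
; Overlapping a MyKey destroys it and prints a message.
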(event Custom|AnimationUpdate
  (if (Variables|Default|GetJustLanded)
    ;[1 1 1] Landing
    (CallFunction|SetFlipBook "NewEnumerator3")
    (Utilities|FlowControl|Delay 0.1)
    (Variables|Default|SetJustLanded false)
    (elif (AI|Components|NavMovement|IsFalling (Variables|Character|GetCharacterMovement))
      (CallFunction|SetFlipBook "NewEnumerator2")
      (else
        ;[1 1 1] running or idle
        (CallFunction|SetFlipBook (select (> (Math|Vector|VectorLength (Transformation|GetVelocity)) 0.0) "NewEnumerator1" "NewEnumerator0"))))))

(event Custom|Direction
  (Math|Float|CompareFloat (.x (Transformation|GetVelocity)) 0.0
    (:>
      ;[1 1 1] facing Right
      (Pawn|SetControlRotation (Pawn|GetController) (Math|Rotator|MakeRotator 0.0 0.0 0.0) :!label _label))
    (:==
      (if (Variables|Default|GetIsMovingRight)
        (goto _label)
        (else
          ;[1 1 1] facing left
          (Pawn|SetControlRotation (Pawn|GetController) (Math|Rotator|MakeRotator 0.0 0.0 1.8e+02) :!label _label_2))))
    (:<
      (goto _label_2))))

(event EventBeginPlay
  (bind _returnvalue (Audio|CreateSound2D "/Game/Audio/jumpSoundCue.jumpSoundCue" 1.0 1.0 0.0 0 false false))
  (bind _output_get (Variables|Default|SetJumpSound _returnvalue))
  (Audio|Components|Audio|Stop _output_get)
  (bind _returnvalue_2 (Audio|CreateSound2D "/Game/Audio/land.land" 1.0 1.0 0.0 0 false false))
  (bind _output_get_2 (Variables|Default|SetLandSound _returnvalue_2))
  (Audio|Components|Audio|Stop _output_get_2))

(event Collision|EventActorBeginOverlap
  (params (OtherActor :type Actor%20Object%20Reference))
  (bind _asmy_key (Utilities|Casting|CastToMyKey OtherActor))
  (Actor|DestroyActor _asmy_key)
  (Development|PrintString "get the key" true true "(R=0.000000,G=0.660000,B=1.000000,A=1.000000)" 1e+01))

(event EventTick
  (params (DeltaSeconds :type Float%20%28single-precision%29))
  (CallFunction|Direction)
  (CallFunction|AnimationUpdate))

(event EventOnLanded
  (params (Hit :type Hit%20Result%20Structure%20%28by%20ref%29))
  (Variables|Default|SetJustLanded (.bblockinghit Hit))
  (Audio|Components|Audio|Play (Variables|Default|GetLandSound) 0.0))

(event Input|ActionEvents|InputActionJump
  (params (Key :type Key%20Structure :default "None"))
  (:Pressed
    (Character|Jump)
    (if (Character|CanJump)
      (Audio|Components|Audio|Play (Variables|Default|GetJumpSound) 0.0)
      (CallFunction|SetFlipBook "NewEnumerator3")
      (Utilities|FlowControl|Delay 0.1)
      (if (AI|Components|NavMovement|IsFalling (Variables|Character|GetCharacterMovement))
        (CallFunction|SetFlipBook "NewEnumerator2"))))
  (:Released
    (Character|StopJumping)))

(event Input|AxisEvents|InputAxisMoveRight
  (params (AxisValue :type Float%20%28single-precision%29))
  (Math|Float|CompareFloat AxisValue 0.0
    (:>
      (Variables|Default|SetIsMovingRight true))
    (:<
      (Variables|Default|SetIsMovingRight false)))
  (Pawn|Input|AddMovementInput "1.000000, 0, 0" AxisValue false))

(fn ConstructionScript)

(fn SetFlipBook
  (params (NextState :type AnimState2D%20Enum :default "NewEnumerator0"))
  (Variables|Default|SetCurrentState NextState)
  (Sprite|SetFlipbook (Variables|Default|GetSprite) (Utilities|Select :Index (Variables|Default|GetCurrentState) :NewEnumerator0 "/Game/PlayerAssets/idle.idle" :NewEnumerator1 "/Game/PlayerAssets/run.run" :NewEnumerator2 "/Game/PlayerAssets/Fall.Fall" :NewEnumerator3 "/Game/PlayerAssets/Jump_Land.Jump_Land")))